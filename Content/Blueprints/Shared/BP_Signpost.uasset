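; BP_Signpost is a shared signpost actor that displays up to six configurable lines of text: a title, a description and four further lines.
; Its construction script fills one text render component per line and destroys the component of any line left empty.
; It then applies the TextColour setting to the first five components, leaving the sixth line's colour unchanged.
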(fn `UserConstructionScript`
  (bind _title (`self.Title`))
  (bind _textrender1 (`self.TextRender1`))
  (bind _textrender4 (`self.TextRender4`))
  (bind _textrender3 (`self.TextRender3`))
  (bind _textrender2 (`self.TextRender2`))
  (bind _line4 (`self.Line4`))
  (bind _line3 (`self.Line3`))
  (bind _description (`self.Description`))
  (bind _line5 (`self.Line5`))
  (bind _textrender5 (`self.TextRender5`))
  (bind _line6 (`self.Line6`))
  (bind _textrender6 (`self.TextRender6`))
  (`|ExecutionSequence`
    (:`then_0`
      (if (== (`KismetStringLibrary.Len` _title) 0)
        (`ActorComponent.K2_DestroyComponent` _textrender1)
        (else
          (`TextRenderComponent.SetText` _textrender1 _title))))
    (:`then_1`
      (if (== (`KismetStringLibrary.Len` _description) 0)
        (`ActorComponent.K2_DestroyComponent` _textrender2)
        (else
          (`TextRenderComponent.SetText` _textrender2 _description))))
    (:`then_2`
      (if (== (`KismetStringLibrary.Len` _line3) 0)
        (`ActorComponent.K2_DestroyComponent` _textrender3)
        (else
          (`TextRenderComponent.SetText` _textrender3 _line3))))
    (:`then_3`
      (if (== (`KismetStringLibrary.Len` _line4) 0)
        (`ActorComponent.K2_DestroyComponent` _textrender4)
        (else
          (`TextRenderComponent.SetText` _textrender4 _line4))))
    (:`then_4`
      (if (== (`KismetStringLibrary.Len` _line5) 0)
        (`ActorComponent.K2_DestroyComponent` _textrender5)
        (else
          (`TextRenderComponent.SetText` _textrender5 _line5))))
    (:`then_5`
      (if (== (`KismetStringLibrary.Len` _line6) 0)
        (`ActorComponent.K2_DestroyComponent` _textrender6)
        (else
          (`TextRenderComponent.SetText` _textrender6 _line6))))
    (:`then_6`
      (`TextRenderComponent.SetTextRenderColor` (`self.TextRender1`) (`KismetMathLibrary.Conv_LinearColorToColor` (`self.TextColour`)))
      (`TextRenderComponent.SetTextRenderColor` (`self.TextRender2`) (`KismetMathLibrary.Conv_LinearColorToColor` (`self.TextColour`)))
      (`TextRenderComponent.SetTextRenderColor` (`self.TextRender3`) (`KismetMathLibrary.Conv_LinearColorToColor` (`self.TextColour`)))
      (`TextRenderComponent.SetTextRenderColor` (`self.TextRender4`) (`KismetMathLibrary.Conv_LinearColorToColor` (`self.TextColour`)))
      (`TextRenderComponent.SetTextRenderColor` (`self.TextRender5`) (`KismetMathLibrary.Conv_LinearColorToColor` (`self.TextColour`))))))