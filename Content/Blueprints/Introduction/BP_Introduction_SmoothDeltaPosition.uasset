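; Introduction example Blueprint that shows smoothed Kinect wrist movement for the centered player as text and arrows.
; Each tick it gets the centered body, reads left and right wrist joint delta positions, and averages each over recent samples.
; A shared helper writes each averaged vector and its rounded length as speed to text components, then rotates an arrow along that direction with a roll offset.
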(event `self.ReceiveTick`
  (params (DeltaSeconds :type "Float (single-precision)"))
  ;[1 1 1] Get dominant player reference
  (bind _centeredbody (`KinectInterfaceComponent.GetCenteredBody` (`self.KinectInterface`)))
  (set `self.CentredBody` _centeredbody)
  ;[1 1 1] Left Wrist display
  (bind _returnvalue (`KinectInterfaceComponent.GetJointDeltaPosition` (`self.KinectInterface`) "WristLeft" (`self.CentredBody`)))
  (bind _average (`/Game/Blueprints/Shared/BPL_MacroLibrary.AverageVectorSamples` _returnvalue)
    (:`Out`
      (`self.SetDisplayComponents` _average (`self.TextLWristCoord`) (`self.TextLWristSpeed`) (`self.ArrowLWrist`))
      ;[1 1 1] Right Wrist display
      (bind _returnvalue_2 (`KinectInterfaceComponent.GetJointDeltaPosition` (`self.KinectInterface`) "WristRight" (`self.CentredBody`)))
      (bind _average_2 (`/Game/Blueprints/Shared/BPL_MacroLibrary.AverageVectorSamples` _returnvalue_2)
        (:`Out`
          (`self.SetDisplayComponents` _average_2 (`self.TextRWristCoord`) (`self.TextRWristSpeed`) (`self.ArrowRWrist`)))))))

(fn `SetDisplayComponents`
  (params (Vector :type "Object.Vector Structure") (TextCoord :type "TextRenderComponent Object Reference") (TextSpeed :type "TextRenderComponent Object Reference") (Arrow :type "SceneComponent Object Reference"))
  (`TextRenderComponent.SetText` TextCoord (`KismetStringLibrary.Conv_VectorToString` Vector))
  (`TextRenderComponent.SetText` TextSpeed (`KismetStringLibrary.Concat_StrStr` "Speed: " (`KismetStringLibrary.Conv_IntToString` (`KismetMathLibrary.Round` (`KismetMathLibrary.VSize` Vector)))))
  (`SceneComponent.K2_SetRelativeRotation` Arrow (`KismetMathLibrary.ComposeRotators` (`KismetMathLibrary.Conv_VectorToRotator` Vector) (struct :`Yaw` 180.0)) false))

(fn `UserConstructionScript`)