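; BP_RobotArms mirrors a Kinect user's left and right hand positions onto two hand components.
; Each Tick it gets the centered body from the Kinect interface and passes it to LHandTracking and RHandTracking.
; These scale each hand joint's absolute position, rotate it -90 degrees in yaw, and set it as relative location without sweep.
; A hit on the right hand component only prints a debug message.
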(event `self.SM_RHand.OnComponentHit`
  (params (OtherActor :type "Actor Object Reference") (OtherComp :type "PrimitiveComponent Object Reference") (NormalImpulse :type "Object.Vector Structure") (Hit :type "EngineTypes.HitResult Structure (by ref)"))
  (`KismetSystemLibrary.PrintString` "ARM ACTIVATED"))

(event `self.ReceiveTick`
  (params (DeltaSeconds :type "Float (single-precision)"))
  ;[1 1 1] Get Centered Body Number
  (bind _centeredbody (`KinectInterfaceComponent.GetCenteredBody` (`self.KinectInterface`)))
  ;[1 1 1] Do Hand Tracking
  (`self.LHandTracking` _centeredbody)
  (`self.RHandTracking` _centeredbody))

(fn `LHandTracking`
  (params (`Body Number` :type Byte))
  ;[1 1 1] Get Joint Position and Convert to Sphere Location
  (bind _returnvalue (`KinectInterfaceComponent.GetJointAbsolutePosition` (`self.KinectInterface`) "HandLeft" (cast `EBodyNumber` `Body Number`)))
  (`SceneComponent.K2_SetRelativeLocation` (`self.SM_LHand`) (`KismetMathLibrary.GreaterGreater_VectorRotator` (* _returnvalue 5.0) (struct :`Yaw` -90.0)) false))

(fn `RHandTracking`
  (params (`Body Number` :type Byte))
  ;[1 1 1] Get Joint Position and Convert to Sphere Location
  (bind _returnvalue (`KinectInterfaceComponent.GetJointAbsolutePosition` (`self.KinectInterface`) "HandRight" (cast `EBodyNumber` `Body Number`)))
  (`SceneComponent.K2_SetRelativeLocation` (`self.SM_RHand`) (`KismetMathLibrary.GreaterGreater_VectorRotator` (* _returnvalue 5.0) (struct :`Yaw` -90.0)) false))

(fn `UserConstructionScript`)